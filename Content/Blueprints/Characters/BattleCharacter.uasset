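; BattleCharacter is a sprite-based character Blueprint for battles, with stub functions for player and enemy actions.
; Each tick it billboards the sprite by yaw only, using the look-at angle from the camera to the capsule plus a 90-degree offset.
; PlayerAction and EnemyAction pass the player and enemy stat sets through unchanged, ignoring the current combatant.
; Crabbler only prints its name, and the construction script is empty.
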(event EventTick
  (params (DeltaSeconds :type Float%20%28single-precision%29))
  ;[1 1 1] Make sprite face camera
  (Transformation|SetRelativeRotation (Variables|Default|GetSprite) (Math|Rotator|MakeRotator 0.0 0.0 (+ (.Yaw (Math|Rotator|BreakRotator (Math|Rotator|FindLookatRotation (Camera|GetCameraLocation (Game|GetPlayerCameraManager 0)) (Transformation|GetWorldLocation (Variables|Collision|GetCapsuleComponent))))) 9e+01)) false false))

(fn ConstructionScript)

(fn Crabbler
  (Development|PrintString "Crabbler"))

(fn PlayerAction
  (params (CurrentPlayerStats :type Stats%20Structure) (AllPlayerStats :type Array%20of%20Stats%20Structures) (AllEnemyStats :type Array%20of%20Stats%20Structures) (CurrentPlayerIndex :type Integer))
  (Variables|Default|SetPlayerStats AllPlayerStats)
  (Variables|Default|SetEnemyStats AllEnemyStats))

(fn EnemyAction
  (params (CurrentEnStats :type Stats%20Structure) (AllPlayerStats :type Array%20of%20Stats%20Structures) (AllEnemyStats :type Array%20of%20Stats%20Structures) (CurrentEnIndex :type Integer))
  (Variables|Default|SetPlayerStats AllPlayerStats)
  (Variables|Default|SetEnemyStats AllEnemyStats))