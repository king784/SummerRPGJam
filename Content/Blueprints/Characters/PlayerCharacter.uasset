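; Player character for field maps: a flipbook sprite that walks or runs in four directions, height-snapped to the ground by a per-tick downward trace.
; BeginPlay restores spawn point and facing from the game instance and creates the dialogue widget.
; Action messages overlapping interactables and opens quest widgets for Quest actors attached to the prompted target.
; Menu toggles the quest log, while capsule overlaps trigger level changes through an interface.
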(event OnComponentBeginOverlap(InteractionField)
  (params (OverlappedComponent :type Primitive%20Component%20Object%20Reference) (OtherActor :type Actor%20Object%20Reference) (OtherComp :type Primitive%20Component%20Object%20Reference) (OtherBodyIndex :type Integer) (bFromSweep :type Boolean) (SweepResult :type Hit%20Result%20Structure%20%28by%20ref%29))
  ;[1 1 1] when something touches the interaction field collision
  ;[1 1 1] Make the interact mesage widget
  (bind _returnvalue (AddComponent|AddWidgetComponent false))
  (Variables|Default|SetInteractMessage _returnvalue)
  (Transformation|AttachComponentToComponent _returnvalue OtherComp "None" "KeepRelative" "KeepRelative" "KeepRelative" true))

(event OnComponentEndOverlap(InteractionField)
  (params (OverlappedComponent :type Primitive%20Component%20Object%20Reference) (OtherActor :type Actor%20Object%20Reference) (OtherComp :type Primitive%20Component%20Object%20Reference) (OtherBodyIndex :type Integer))
  ;[1 1 1] when that somehting leaves the interaction field
  ;[1 1 1] if the interact message is being displayed, destroy it
  (bind _interactmessage (Variables|Default|GetInteractMessage)
    (:then
      (Components|DestroyComponent _interactmessage)
      ;[1 1 1] then set it as empty
      (Variables|Default|SetInteractMessage 0))
    (:else)))

(event OnComponentBeginOverlap(CapsuleComponent)
  (params (OverlappedComponent :type Primitive%20Component%20Object%20Reference) (OtherActor :type Actor%20Object%20Reference) (OtherComp :type Primitive%20Component%20Object%20Reference) (OtherBodyIndex :type Integer) (bFromSweep :type Boolean) (SweepResult :type Hit%20Result%20Structure%20%28by%20ref%29))
  ;[1 1 1] Change level when hit door
  (if (Utilities|DoesObjectImplementInterface OtherActor "/Game/Blueprints/ChangeLevelInterface.ChangeLevelInterface_C")
    (Class|ChangeLevelInterface|ChangeLevel(Message) OtherActor)))

(event Custom|GetEventRef
  (params (NewNPCRef :type NPC%20Character%20Object%20Reference))
  (Variables|Default|SetEventRef NewNPCRef))

(event EventBeginPlay
  (Utilities|Array|Clear (Variables|Default|GetAllPlayerStarts))
  (bind _outactors (Actor|GetAllActorsOfClass "/Script/Engine.PlayerStart"))
  (Variables|Default|SetAllPlayerStarts _outactors)
  (bind _asmy_game_instance (Utilities|Casting|CastToMyGameInstance (Game|GetGameInstance)))
  (bind _array_element (Utilities|Array|ForEachLoopwithBreak (Variables|Default|GetAllPlayerStarts) :!label _label)
    (:LoopBody
      (if (Utilities|Name|Equal(Name) (Variables|/Script/Engine.PlayerStart|GetPlayerStartTag _array_element) (Utilities|String|StringToName (Utilities|String|ToString(Integer) (Variables|/Game/Blueprints/MyGameInstance.MyGameInstance_C|GetNextPlayerStartIndex _asmy_game_instance))))
        (Transformation|Teleport (Transformation|GetActorLocation _array_element) "0, 0, 0")
        (goto _label Break)))
    (:Completed
      (Variables|Default|SetDirection (Variables|/Game/Blueprints/MyGameInstance.MyGameInstance_C|GetPlayerFieldStartDirection _asmy_game_instance))
      (bind _returnvalue (UserInterface|CreateWidget "/Game/Dialogue/DialogueWidget.DialogueWidget_C" (Game|GetPlayerController 0)))
      (bind _output_get (Variables|Default|SetDialogueWidgetRef _returnvalue))
      (UserInterface|Viewport|AddtoViewport _output_get 0))))

(event EventTick
  (params (DeltaSeconds :type Float%20%28single-precision%29))
  (CallFunction|SetDirection)
  (CallFunction|CalculateZ))

(event Input|ActionEvents|InputActionAction
  (params (Key :type Key%20Structure))
  (:Pressed
    ;[1 1 1] check if interactmessage exists
    (bind _interactmessage (Variables|Default|GetInteractMessage)
      (:then
        ;[1 1 1] get all children actors from parent and loop through them
        (for _array_element (Actor|GetAttachedActors (Components|GetOwner (Transformation|GetAttachParent _interactmessage)))
          ;[1 1 1] cast child element as quest and if valid add quest ui as a child of game mode's hud canvas
          (bind _asquest (Utilities|Casting|CastToQuest _array_element))
          (bind _returnvalue (UserInterface|CreateWidget "/Game/QuestSystem/QuestUI/Quest_UI.Quest_UI_C" 0 _asquest))
          (bind _asfield_game_mode (Utilities|Casting|CastToFieldGameMode (Game|GetGameMode)))
          (bind _returnvalue_2 (Class|CanvasPanel|AddChildtoCanvas (Variables|/Game/HUD/HUD_UI.HUD_UI_C|GetQuestDoialogueHolder (Variables|/Game/Blueprints/GameModes/FieldGameMode.FieldGameMode_C|GetHUD_Widget _asfield_game_mode)) _returnvalue))
          (Class|CanvasPanelSlot|SetAutoSize _returnvalue_2 true)))
      (:else))))

(event Input|ActionEvents|InputActionAction
  (params (Key :type Key%20Structure))
  (:Pressed
    (bind _outactors (Actor|GetAllActorswithInterface "/Game/Blueprints/InteractInterface.InteractInterface_C"))
    (bind _array_element (Utilities|Array|ForEachLoopwithBreak _outactors :!label _label)
      (:LoopBody
        (if (Collision|IsOverlappingActor _array_element self :!class /Script/Engine.Actor)
          (Class|InteractInterface|Interact(Message) _array_element)
          (goto _label Break))))))

(event Input|ActionEvents|InputActionCancel
  (params (Key :type Key%20Structure))
  (bind _charactermovement (Variables|Character|GetCharacterMovement))
  (:Pressed
    (Variables|/Script/Engine.CharacterMovementComponent|SetMaxFlySpeed _charactermovement 7.5e+02)
    (Variables|Default|SetisRunning true))
  (:Released
    (Variables|/Script/Engine.CharacterMovementComponent|SetMaxFlySpeed _charactermovement 4e+02)
    (Variables|Default|SetisRunning false)))

(event Input|ActionEvents|InputActionMenu
  (params (Key :type Key%20Structure))
  (:Pressed
    ;[1 1 1] check if questlog widget already exists
    (bind _questlogui (Variables|Default|GetQuestLogUI)
      (:then
        ;[1 1 1] set the widget as empty
        (Widget|RemovefromParent _questlogui)
        (Variables|Default|SetQuestLogUI 0))
      (:else
        ;[1 1 1] create quest log widget
        (bind _returnvalue (UserInterface|CreateWidget "/Game/QuestSystem/QuestUI/QuestLog_UI.QuestLog_UI_C"))
        (Variables|Default|SetQuestLogUI _returnvalue)
        ;[1 1 1] Get the game mode and the hud canvas from there
        (bind _asfield_game_mode (Utilities|Casting|CastToFieldGameMode (Game|GetGameMode)))
        ;[1 1 1] add questlog widget to canvas as a child and set its anchors
        (bind _returnvalue_2 (Class|CanvasPanel|AddChildtoCanvas (Variables|/Game/Blueprints/GameModes/FieldGameMode.FieldGameMode_C|GetHUD_Canvas _asfield_game_mode) (Variables|Default|GetQuestLogUI)))
        (Class|CanvasPanelSlot|SetAnchors _returnvalue_2 (Utilities|Struct|MakeAnchors "(X=0.000000,Y=0.000000)" "(X=1.000000,Y=1.000000)"))))))

(event Input|AxisEvents|InputAxisXAxis
  (params (AxisValue :type Float%20%28single-precision%29))
  (Pawn|Input|AddMovementInput "0.000000,1.000000, 0" AxisValue false))

(event Input|AxisEvents|InputAxisYAxis
  (params (AxisValue :type Float%20%28single-precision%29))
  (Pawn|Input|AddMovementInput "-1.000000, 0, 0" AxisValue false))

(fn ConstructionScript
  (Transformation|SetWorldRotation (Variables|Default|GetSprite) (Math|Rotator|MakeRotator (.pitch (Transformation|GetWorldRotation (Variables|Default|GetSpringArm1))) 0.0 -9e+01) false false))

(fn SetDirection
  (bind _sprite (Variables|Default|GetSprite))
  (bind _sprite_2 (Variables|Default|GetSprite))
  (if (or (!= (Input|AxisValues|GetXAxis) 0.0) (!= (Input|AxisValues|GetYAxis) 0.0))
    (Variables|Default|SetDirection (select (> (Input|AxisValues|GetYAxis) 0.0) "NewEnumerator0" (select (< (Input|AxisValues|GetYAxis) 0.0) "NewEnumerator1" (select (> (Input|AxisValues|GetXAxis) 0.0) "NewEnumerator2" "NewEnumerator3"))))
    (if (Variables|Default|GetisRunning)
      (Sprite|SetFlipbook _sprite (Utilities|Select :Index (Variables|Default|GetDirection) :NewEnumerator0 "/Game/Textures/Player/Box/MoveUp.MoveUp" :NewEnumerator1 "/Game/Textures/Player/Box/MoveDown.MoveDown" :NewEnumerator2 "/Game/Textures/Player/Box/MoveLeft.MoveLeft" :NewEnumerator3 "/Game/Textures/Player/Box/MoveRight.MoveRight"))
      (Components|Timeline|SetPlayRate _sprite_2 2.0)
      (else
        (Sprite|SetFlipbook _sprite (Utilities|Select :Index (Variables|Default|GetDirection) :NewEnumerator0 "/Game/Textures/Player/Box/MoveUp.MoveUp" :NewEnumerator1 "/Game/Textures/Player/Box/MoveDown.MoveDown" :NewEnumerator2 "/Game/Textures/Player/Box/MoveLeft.MoveLeft" :NewEnumerator3 "/Game/Textures/Player/Box/MoveRight.MoveRight"))
        (Components|Timeline|SetPlayRate _sprite_2 1.0)))
    (else
      (Sprite|SetFlipbook _sprite (select (> (Math|Vector|VectorLength (Transformation|GetVelocity)) 0.0) (Utilities|Select :Index (Variables|Default|GetDirection) :NewEnumerator0 "/Game/Textures/Player/Box/MoveUp.MoveUp" :NewEnumerator1 "/Game/Textures/Player/Box/MoveDown.MoveDown" :NewEnumerator2 "/Game/Textures/Player/Box/MoveLeft.MoveLeft" :NewEnumerator3 "/Game/Textures/Player/Box/MoveRight.MoveRight") (Utilities|Select :Index (Variables|Default|GetDirection) :NewEnumerator0 "/Game/Textures/Player/Box/IdleUp.IdleUp" :NewEnumerator1 "/Game/Textures/Player/Box/IdleDown.IdleDown" :NewEnumerator2 "/Game/Textures/Player/Box/IdleLeft.IdleLeft" :NewEnumerator3 "/Game/Textures/Player/Box/IdleRight.IdleRight"))))))

(fn CalculateZ
  (bind _returnvalue (Transformation|GetActorLocation))
  (bind _returnvalue_2 (Transformation|GetActorLocation))
  (bind _outhit (Collision|LineTraceByChannel (Transformation|GetActorLocation) (Math|Vector|MakeVector (.x _returnvalue) (.y _returnvalue) (- (.z _returnvalue) 2e+02)) "TraceTypeQuery1" false 0 "None"))
  (Transformation|SetActorLocation (Math|Vector|MakeVector (.x _returnvalue_2) (.y _returnvalue_2) (+ (.z (.ImpactPoint (Collision|BreakHitResult _outhit))) (Variables|Default|GetDistanceZ))) false false))