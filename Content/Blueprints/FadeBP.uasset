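; FadeBP is an actor Blueprint that drives a full-screen fade, fading in automatically when play begins.
; BeginPlay adds a FadeWidget to player 0's viewport and stores the dynamic material of its FadeImg.
; FadeIn and FadeOut use separate timelines, each writing a FadeToBlack track to the material's Alpha parameter.
; FadeIn plays its timeline in reverse from the end, while FadeOut plays forward.
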(event Custom|FadeOut
  (bind _fadetoblack (Timeline|Timeline_2 Play)
    (:Update
      (Rendering|Material|SetScalarParameterValue (Variables|Default|GetFadeMat) "Alpha" _fadetoblack :!class /Script/Engine.MaterialInstanceDynamic))))

(event Custom|FadeIn
  (bind _fadetoblack (Timeline|Timeline_1 ReverseFromEnd)
    (:Update
      (Rendering|Material|SetScalarParameterValue (Variables|Default|GetFadeMat) "Alpha" _fadetoblack :!class /Script/Engine.MaterialInstanceDynamic))))

(event EventBeginPlay
  (bind _returnvalue (UserInterface|CreateWidget "/Game/Blueprints/FadeWidget.FadeWidget_C" (Game|GetPlayerController 0)))
  (UserInterface|Viewport|AddtoViewport _returnvalue 0)
  (bind _returnvalue_2 (Appearance|GetDynamicMaterial (Variables|/Game/Blueprints/FadeWidget.FadeWidget_C|GetFadeImg _returnvalue) :!class /Script/UMG.Image))
  (Variables|Default|SetFadeMat _returnvalue_2)
  (CallFunction|Fadein))

(fn ConstructionScript)