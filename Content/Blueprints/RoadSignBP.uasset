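; RoadSignBP is a road sign that shows its LocationsText in a dialogue widget when interacted with.
; Interact toggles the display: it removes and clears an existing widget, or creates a DialogueWidget for player controller 0, adds it to the viewport and sets its text.
; The Trigger end-overlap event and the construction script are empty, so leaving the trigger does not close the dialogue.
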(event OnComponentEndOverlap(Trigger)
  (params (OverlappedComponent :type Primitive%20Component%20Object%20Reference) (OtherActor :type Actor%20Object%20Reference) (OtherComp :type Primitive%20Component%20Object%20Reference) (OtherBodyIndex :type Integer)))

(event EventInteract
  (params (Interacter :type Actor%20Object%20Reference))
  (Utilities|IsValid (Variables|Default|GetDialogueWidgetRef)
    (:Is%20Valid
      (Widget|RemovefromParent (Variables|Default|GetDialogueWidgetRef))
      (Variables|Default|SetDialogueWidgetRef 0))
    (:Is%20Not%20Valid
      (bind _returnvalue (UserInterface|CreateWidget "/Game/Dialogue/DialogueWidget.DialogueWidget_C" (Game|GetPlayerController 0)))
      (bind _output_get (Variables|Default|SetDialogueWidgetRef _returnvalue))
      (UserInterface|Viewport|AddtoViewport _output_get 0)
      (Variables|/Game/Dialogue/DialogueWidget.DialogueWidget_C|SetDialogue _output_get (Variables|Default|GetLocationsText))
      (Widget|SetVisibility _output_get "Visible"))))

(fn ConstructionScript)