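; Paper2D NPC that can wander random navmesh points and talk to the player.
; BeginPlay gathers its name and rows from the Dialogue DataTable by NPCID; Interact steps through conversation lines in a DialogueWidget, removed when lines run out or the player leaves.
; Tick snaps it to the ground by downward trace and rotates the sprite to the player's spring-arm pitch.
; SetDirection picks directional flipbooks but is not called here.
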(event OnComponentBeginOverlap(EventTrigger)
  (params (OverlappedComponent :type Primitive%20Component%20Object%20Reference) (OtherActor :type Actor%20Object%20Reference) (OtherComp :type Primitive%20Component%20Object%20Reference) (OtherBodyIndex :type Integer) (bFromSweep :type Boolean) (SweepResult :type Hit%20Result%20Structure%20%28by%20ref%29))
  ;[1 1 1] Overlap
)

(event OnComponentEndOverlap(EventTrigger)
  (params (OverlappedComponent :type Primitive%20Component%20Object%20Reference) (OtherActor :type Actor%20Object%20Reference) (OtherComp :type Primitive%20Component%20Object%20Reference) (OtherBodyIndex :type Integer))
  (Utilities|Casting|CastToPlayerCharacter OtherActor)
  (Variables|/Script/Engine.CharacterMovementComponent|SetMaxFlySpeed (Variables|Character|GetCharacterMovement) 2e+02)
  (Utilities|IsValid (Variables|Default|GetDialogueWidgetRef)
    (:Is%20Valid
      (Widget|RemovefromParent (Variables|Default|GetDialogueWidgetRef))
      (Variables|Default|SetDialogueWidgetRef 0))))

(event Custom|WalkEvent
  ;[1 1 1] Walk
  (if (not (Variables|Default|GetisWalking))
    (AI|AIMoveTo self (.RandomLocation (Class|NavigationSystemV1|GetRandomPointinNavigableRadius (Transformation|GetActorLocation) (Variables|Default|GetWalkRadius) 0 0)) 0 5.0 false
      (:then
        (Variables|Default|SetisWalking true))
      (:OnSuccess
        (Utilities|FlowControl|Delay (Variables|Default|GetWalkDelay) :!label _label)
        (Variables|Default|SetisWalking false)
        (CallFunction|WalkEvent))
      (:OnFail
        (goto _label)))))

(event EventInteract
  (Math|Integer|IncrementInt (Variables|Default|GetLineCurrent)
    (:%20%20
      (CallFunction|DialogueCreate)
      (Variables|/Script/Engine.CharacterMovementComponent|SetMaxFlySpeed (Variables|Character|GetCharacterMovement) 0.0))))

(event EventTick
  (params (DeltaSeconds :type Float%20%28single-precision%29))
  ;[1 1 1] Event Tick
  (CallFunction|CalculateZ)
  (Transformation|SetWorldRotation (Variables|Default|GetSprite) (Math|Rotator|MakeRotator (.pitch (Transformation|GetWorldRotation (Variables|/Game/Blueprints/PlayerCharacter.PlayerCharacter_C|GetSpringArm1 (Variables|Default|GetCharObjRef)))) 0.0 -9e+01) false false))

(event EventBeginPlay
  (bind _asplayer_character (Utilities|Casting|CastToPlayerCharacter (Game|GetPlayerCharacter 0)))
  (Variables|Default|SetCharObjRef _asplayer_character)
  (if (Variables|Default|GetPatrol)
    (CallFunction|WalkEvent))
  (bind _outrownames (DataTable|GetDataTableRowNames "/Game/Dialogue/Dialogue.Dialogue"))
  (bind _array_element (Utilities|Array|ForEachLoopwithBreak _outrownames :!label _label)
    (:LoopBody
      (bind _returnvalue (Utilities|GetDataTableRow "/Game/Dialogue/Dialogue.Dialogue" _array_element)
        (:then
          (if (== (.NPC_ID (Utilities|Struct|BreakDialogueStructure _returnvalue)) (Variables|Default|GetNPC_ID))
            (if (Utilities|Text|TextIsEmpty (Variables|Default|GetMyName))
              (Variables|Default|SetMyName (.NPCName (Utilities|Struct|BreakDialogueStructure _returnvalue)))
              (goto _label Break))))))
    (:Completed
      (bind _outrownames_2 (DataTable|GetDataTableRowNames "/Game/Dialogue/Dialogue.Dialogue"))
      (for _array_element_2 _outrownames_2
        (bind _returnvalue_2 (Utilities|GetDataTableRow "/Game/Dialogue/Dialogue.Dialogue" _array_element_2)
          (:then
            (if (== (.NPC_ID (Utilities|Struct|BreakDialogueStructure _returnvalue_2)) (Variables|Default|GetNPC_ID))
              (Utilities|Array|Add (Variables|Default|GetMyDialogue) _array_element_2))))))))

(fn ConstructionScript)

(fn SetDirection
  (bind _sprite (Variables|Default|GetSprite))
  (bind _sprite_2 (Variables|Default|GetSprite))
  (if (or (!= (Input|AxisValues|GetXAxis) 0.0) (!= (Input|AxisValues|GetYAxis) 0.0))
    (Variables|Default|SetDirection (select (> (Input|AxisValues|GetYAxis) 0.0) "NewEnumerator0" (select (< (Input|AxisValues|GetYAxis) 0.0) "NewEnumerator1" (select (> (Input|AxisValues|GetXAxis) 0.0) "NewEnumerator2" "NewEnumerator3"))))
    (if (Variables|Default|GetisWalking)
      (Sprite|SetFlipbook _sprite (Utilities|Select :Index (Variables|Default|GetDirection) :NewEnumerator0 "/Game/Textures/Player/Box/MoveUp.MoveUp" :NewEnumerator1 "/Game/Textures/Player/Box/MoveDown.MoveDown" :NewEnumerator2 "/Game/Textures/Player/Box/MoveLeft.MoveLeft" :NewEnumerator3 "/Game/Textures/Player/Box/MoveRight.MoveRight"))
      (Components|Timeline|SetPlayRate _sprite_2 2.0)
      (else
        (Sprite|SetFlipbook _sprite (Utilities|Select :Index (Variables|Default|GetDirection) :NewEnumerator0 "/Game/Textures/Player/Box/MoveUp.MoveUp" :NewEnumerator1 "/Game/Textures/Player/Box/MoveDown.MoveDown" :NewEnumerator2 "/Game/Textures/Player/Box/MoveLeft.MoveLeft" :NewEnumerator3 "/Game/Textures/Player/Box/MoveRight.MoveRight"))
        (Components|Timeline|SetPlayRate _sprite_2 1.0)))
    (else
      (Sprite|SetFlipbook _sprite (select (> (Math|Vector|VectorLength (Transformation|GetVelocity)) 0.0) (Utilities|Select :Index (Variables|Default|GetDirection) :NewEnumerator0 "/Game/Textures/Player/Box/MoveUp.MoveUp" :NewEnumerator1 "/Game/Textures/Player/Box/MoveDown.MoveDown" :NewEnumerator2 "/Game/Textures/Player/Box/MoveLeft.MoveLeft" :NewEnumerator3 "/Game/Textures/Player/Box/MoveRight.MoveRight") (Utilities|Select :Index (Variables|Default|GetDirection) :NewEnumerator0 "/Game/Textures/Player/Box/IdleUp.IdleUp" :NewEnumerator1 "/Game/Textures/Player/Box/IdleDown.IdleDown" :NewEnumerator2 "/Game/Textures/Player/Box/IdleLeft.IdleLeft" :NewEnumerator3 "/Game/Textures/Player/Box/IdleRight.IdleRight"))))))

(fn CalculateZ
  (bind _returnvalue (Transformation|GetActorLocation))
  (bind _returnvalue_2 (Transformation|GetActorLocation))
  (bind _outhit (Collision|LineTraceByChannel (Transformation|GetActorLocation) (Math|Vector|MakeVector (.x _returnvalue) (.y _returnvalue) (- (.z _returnvalue) 2e+02)) "TraceTypeQuery1" false 0 "None"))
  (Transformation|SetActorLocation (Math|Vector|MakeVector (.x _returnvalue_2) (.y _returnvalue_2) (+ (.z (.ImpactPoint (Collision|BreakHitResult _outhit))) 2e+01)) false false))

(fn DialogueCreate
  (Utilities|IsValid (Variables|Default|GetDialogueWidgetRef)
    (:Is%20Valid
      (bind _returnedline (CallFunction|DialogueGetLine))
      (if (Utilities|Enum|NotEqual(Enum) (Variables|Default|GetEmptyText) _returnedline)
        (Variables|/Game/Dialogue/DialogueWidget.DialogueWidget_C|SetNPCName (Variables|Default|GetDialogueWidgetRef) (Variables|Default|GetMyName))
        (Variables|/Game/Dialogue/DialogueWidget.DialogueWidget_C|SetDialogue (Variables|Default|GetDialogueWidgetRef) _returnedline)
        (Widget|SetVisibility (Variables|Default|GetDialogueWidgetRef) "Visible")))
    (:Is%20Not%20Valid
      (bind _returnvalue (UserInterface|CreateWidget "/Game/Dialogue/DialogueWidget.DialogueWidget_C" (Game|GetPlayerController 0)))
      (bind _output_get (Variables|Default|SetDialogueWidgetRef _returnvalue))
      (UserInterface|Viewport|AddtoViewport _output_get 0)
      (bind _returnedline_2 (CallFunction|DialogueGetLine))
      (Utilities|IsValid (Variables|Default|GetDialogueWidgetRef)
        (:Is%20Valid
          (Variables|/Game/Dialogue/DialogueWidget.DialogueWidget_C|SetNPCName (Variables|Default|GetDialogueWidgetRef) (Variables|Default|GetMyName))
          (Variables|/Game/Dialogue/DialogueWidget.DialogueWidget_C|SetDialogue (Variables|Default|GetDialogueWidgetRef) _returnedline_2)
          (Widget|SetVisibility (Variables|Default|GetDialogueWidgetRef) "Visible"))))))

(fn DialogueGetLine
  (for _array_element (Variables|Default|GetMyDialogue)
    (bind _returnvalue (Utilities|GetDataTableRow "/Game/Dialogue/Dialogue.Dialogue" _array_element)
      (:then
        (if (and (== (.Conversation_ID (Utilities|Struct|BreakDialogueStructure _returnvalue)) (Variables|Default|GetConversation_ID)) (== (.Line_ID (Utilities|Struct|BreakDialogueStructure _returnvalue)) (Variables|Default|GetLineCurrent)))
          (Utilities|Array|Add (LocalVariables|GetReturnedLines) (.Dialogue (Utilities|Struct|BreakDialogueStructure _returnvalue)))))))
  (if (== (Utilities|Array|Length (LocalVariables|GetReturnedLines)) 1)
    (return (Utilities|Array|Get(acopy) (LocalVariables|GetReturnedLines)))
    (else
      (Widget|RemovefromParent (Variables|Default|GetDialogueWidgetRef))
      (Variables|Default|SetDialogueWidgetRef 0)
      (Variables|Default|SetLineCurrent 0))))