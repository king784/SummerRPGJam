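; Treasure chest actor that gives the interacting actor its configured item once and shows a "Found" message with the item name.
; The first Interact opens the chest through its anim blueprint's OpenBool, spawns a dialogue widget and adds one item to the interacter's InventoryComponent.
; Interacting again while the message shows dismisses it, as does the player character leaving the Trigger volume.
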(event OnComponentEndOverlap(Trigger)
  (params (OverlappedComponent :type Primitive%20Component%20Object%20Reference) (OtherActor :type Actor%20Object%20Reference) (OtherComp :type Primitive%20Component%20Object%20Reference) (OtherBodyIndex :type Integer))
  (Utilities|Casting|CastToPlayerCharacter OtherActor)
  (Utilities|IsValid (Variables|Default|GetDialogueWidgetRef)
    (:Is%20Valid
      (Widget|RemovefromParent (Variables|Default|GetDialogueWidgetRef))
      (Variables|Default|SetDialogueWidgetRef 0))))

(event EventInteract
  (params (Interacter :type Actor%20Object%20Reference))
  (Utilities|IsValid (Variables|Default|GetDialogueWidgetRef)
    (:Is%20Valid
      (Widget|RemovefromParent (Variables|Default|GetDialogueWidgetRef))
      (Variables|Default|SetDialogueWidgetRef 0))
    (:Is%20Not%20Valid
      (if (not (Variables|Default|GetHasBeenOpened))
        (Variables|Default|SetHasBeenOpened true)
        (bind _returnvalue (UserInterface|CreateWidget "/Game/Dialogue/DialogueWidget.DialogueWidget_C" (Game|GetPlayerController 0)))
        (bind _output_get (Variables|Default|SetDialogueWidgetRef _returnvalue))
        (UserInterface|Viewport|AddtoViewport _output_get 0)
        (Variables|/Game/Dialogue/DialogueWidget.DialogueWidget_C|SetDialogue _output_get (Utilities|Text|ToText(String) (Utilities|String|Append "Found " (Utilities|String|ToString(Text) (.Name (Utilities|Struct|BreakItemStructure (Variables|Default|GetItem)))))))
        (Widget|SetVisibility _output_get "Visible")
        (bind _astreasure_chest_anim_bp (Utilities|Casting|CastToTreasureChestAnimBP (Components|SkeletalMesh|GetAnimInstance (Variables|Default|GetTreasureChest))))
        (Variables|/Game/Models/TreasureChestAnimBP.TreasureChestAnimBP_C|SetOpenBool _astreasure_chest_anim_bp true)
        (Default|AddtoInventory (Actor|GetComponentbyClass Interacter "/Game/Inventory/InventoryComponent.InventoryComponent_C") (Utilities|Struct|MakeSlotStructure (Variables|Default|GetItem) 1 (.name (Variables|Default|GetItem))))))))

(fn ConstructionScript)