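; Random encounter controller that readies a level's possible battles and launches the battle level as the player moves.
; On BeginPlay it filters the Formations table by area name, gathers matching Monsters rows, and stores both in MyGameInstance.
; It randomizes the encounter threshold, then Tick increments a frame-based counter while player horizontal speed is high enough.
; At the threshold it disables input, triggers FadeBP and immediately opens the battle level.
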(event EventTick
  (params (DeltaSeconds :type Float%20%28single-precision%29))
  (bind _returnvalue (Game|GetPlayerCharacter 0))
  ;[1 1 1] Set values for encounters
  (if (not (<= (Variables|Default|GetNextEncounterValue) 0.0))
    (Utilities|Casting|CastToPlayerCharacter _returnvalue)
    (if (>= (Math|Vector|VectorLengthXY (Transformation|GetVelocity _returnvalue)) 4e+01)
      (Variables|Default|SetCurrentEncounterValue (+ (Variables|Default|GetCurrentEncounterValue) 1.0))
      (if (>= (+ (Variables|Default|GetCurrentEncounterValue) 1.0) (Variables|Default|GetNextEncounterValue))
        (Variables|Default|SetCurrentEncounterValue 0.0)
        (Input|DisableInput (Game|GetPlayerController 0))
        (bind _outactors (Actor|GetAllActorsOfClass "/Game/Blueprints/FadeBP.FadeBP_C"))
        (Utilities|IsValid (Utilities|Array|Get(acopy) _outactors)
          (:Is%20Valid
            (Default|FadeOut (Utilities|Array|Get(acopy) _outactors)))
          (:Is%20Not%20Valid
            _))
        (Game|OpenLevel(byName) (Variables|Default|GetBattleLevelName))))))

(event EventBeginPlay
  ;[1 1 1] Loop and find all battle formations possible in this level
  (bind _outrownames (DataTable|GetDataTableRowNames "/Game/Monsters/Formations.Formations"))
  (bind _array_element (Utilities|Array|ForEachLoopwithBreak _outrownames)
    (:LoopBody
      (bind _returnvalue (Utilities|GetDataTableRow "/Game/Monsters/Formations.Formations" _array_element)
        (:then
          (if (Utilities|Enum|Equal(Enum) (.Level (Utilities|Struct|BreakFormationStruct _returnvalue)) (Utilities|Text|ToText(Name) (Variables|Default|GetCurrentAreaName)))
            (Utilities|Array|Add (Variables|Default|GetPossibleBattleFormations) _returnvalue)))))
    (:Completed
      (bind _asmy_game_instance (Utilities|Casting|CastToMyGameInstance (Game|GetGameInstance))
        (:then
          ;[1 1 1] Look for correct monsters in the formations and add them to possible monsters
          (Variables|/Game/Blueprints/MyGameInstance.MyGameInstance_C|SetBattleFormations _asmy_game_instance (Variables|Default|GetPossibleBattleFormations))
          (bind _outrownames_2 (DataTable|GetDataTableRowNames "/Game/Monsters/Monsters.Monsters"))
          (bind _array_element_2 (Utilities|Array|ForEachLoopwithBreak _outrownames_2)
            (:LoopBody
              (bind _returnvalue_2 (Utilities|GetDataTableRow "/Game/Monsters/Monsters.Monsters" _array_element_2)
                (:then
                  (bind _array_element_3 (Utilities|Array|ForEachLoopwithBreak (Variables|Default|GetPossibleBattleFormations))
                    (:LoopBody
                      (if (Math|Boolean|ORBoolean (Utilities|Enum|Equal(Enum) (.Name (Utilities|Struct|BreakMonsterStruct _returnvalue_2)) (.Monster1 (Utilities|Struct|BreakFormationStruct _array_element_3))) (Utilities|Enum|Equal(Enum) (.Monster2 (Utilities|Struct|BreakFormationStruct _array_element_3)) (.Name (Utilities|Struct|BreakMonsterStruct _returnvalue_2))) (Utilities|Enum|Equal(Enum) (.Monster3 (Utilities|Struct|BreakFormationStruct _array_element_3)) (.Name (Utilities|Struct|BreakMonsterStruct _returnvalue_2))) (Utilities|Enum|Equal(Enum) (.Monster4 (Utilities|Struct|BreakFormationStruct _array_element_3)) (.Name (Utilities|Struct|BreakMonsterStruct _returnvalue_2))) (Utilities|Enum|Equal(Enum) (.Monster5 (Utilities|Struct|BreakFormationStruct _array_element_3)) (.Name (Utilities|Struct|BreakMonsterStruct _returnvalue_2))))
                        (Utilities|Array|Add (Variables|Default|GetPossibleEnemies) _returnvalue_2)))))))
            (:Completed
              ;[1 1 1] Tell the possible enemies to game instance
              (Utilities|Array|Clear (Variables|/Game/Blueprints/MyGameInstance.MyGameInstance_C|GetEnemyParty _asmy_game_instance))
              (for _array_element_4 (Variables|Default|GetPossibleEnemies)
                (Utilities|Array|Add (Variables|/Game/Blueprints/MyGameInstance.MyGameInstance_C|GetEnemyParty _asmy_game_instance) _array_element_4))
              ;[1 1 1] Set values for encounters
              (Variables|Default|SetNextEncounterValue (Math|Random|RandomFloatinRange (- (Variables|Default|GetNextEncounterValue) 2e+01) (+ (Variables|Default|GetNextEncounterValue) 2e+01)) :!label _label)
              (Variables|Default|SetCurrentEncounterValue 0.0))))
        (:CastFailed
          (goto _label))))))

(fn ConstructionScript)