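; BattleManager sets up a battle on BeginPlay, picking a random formation from the game instance and spawning both parties as BattleCharacters at placed spawn actors.
; Player members take spawn points in party order, while enemies match formation monster names, whose trailing character selects the spawn index.
; It switches the view to the battle camera immediately and again when the level start sequence finishes.
; Turn order is only a placeholder comment.
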(event Custom|SetBattleCam
  ;[1 1 1] Set main camera to the battle camera after camera battle opening sequence
  (Game|Player|SetViewTargetwithBlend (Game|GetPlayerController 0) (Variables|Default|GetBattleCamera) 0.0 "VTBlend_Linear" 0.0 false) ; Turn order after this!!
)

(event EventBeginPlay
  (bind _enemyspawnactors (Variables|Default|GetEnemySpawnActors))
  ;[1 1 1] Randomize battleformation
  (bind _asmy_game_instance (Utilities|Casting|CastToMyGameInstance (Game|GetGameInstance)))
  (Variables|Default|SetBattleFormation (Utilities|Array|Get(acopy) (Variables|/Game/Blueprints/MyGameInstance.MyGameInstance_C|GetBattleFormations _asmy_game_instance) (Math|Random|RandomIntegerinRange 0 (- (Utilities|Array|Length (Variables|/Game/Blueprints/MyGameInstance.MyGameInstance_C|GetBattleFormations _asmy_game_instance)) 1))))
  (CallFunction|SetBattleCam)
  ;[1 1 1] Set player party locations
  (for (_ _array_index) (Variables|Default|GetPlayerSpawnActors)
    (Utilities|Array|Add (Variables|Default|GetPlayerSpawnPoints) (Transformation|GetActorTransform (Utilities|Array|Get(acopy) (Variables|Default|GetPlayerSpawnActors) _array_index))))
  (for (_ _array_index_2) (Variables|/Game/Blueprints/MyGameInstance.MyGameInstance_C|GetBattleParty _asmy_game_instance)
    (Game|SpawnActorfromClass "/Game/Blueprints/Characters/BattleCharacter.BattleCharacter_C" (Math|Transform|MakeTransform (+ (.location (Utilities|Array|Get(acopy) (Variables|Default|GetPlayerSpawnPoints) _array_index_2)) "0, 0,2.000000") "0, 0, 0" "1,1,1") "AdjustIfPossibleButAlwaysSpawn" 0 0))
  ;[1 1 1] Set enemies to correct locations and set the flipbook
  (for (_ _array_index_3) _enemyspawnactors
    (Utilities|Array|Add (Variables|Default|GetEnemySpawnPoints) (Transformation|GetActorTransform (Utilities|Array|Get(acopy) _enemyspawnactors _array_index_3))))
  (for _index (range 0 4)
    (bind _array_element (Utilities|Array|ForEachLoopwithBreak (Variables|/Game/Blueprints/MyGameInstance.MyGameInstance_C|GetEnemyParty _asmy_game_instance))
      (:LoopBody
        (if (and (not (Utilities|Text|TextIsEmpty (.Name (Utilities|Struct|BreakMonsterStruct _array_element)))) (and (Utilities|Enum|Equal(Enum) (.Name (Utilities|Struct|BreakMonsterStruct _array_element)) (.Monster1 (Utilities|Struct|BreakFormationStruct (Variables|Default|GetBattleFormation)))) (== _index (Utilities|GetLastLetterMacro (.Monster1 (Utilities|Struct|BreakFormationStruct (Variables|Default|GetBattleFormation)))))))
          (bind _returnvalue (Game|SpawnActorfromClass "/Game/Blueprints/Characters/BattleCharacter.BattleCharacter_C" (Math|Transform|MakeTransform (+ (.Location (Math|Transform|BreakTransform (Utilities|Array|Get(acopy) (Variables|Default|GetEnemySpawnPoints) _index))) "0, 0,2.000000") "0, 0, 0" "1,1,1") "AdjustIfPossibleButAlwaysSpawn" 0 0 :!label _label))
          (Sprite|SetFlipbook (Variables|/Script/Paper2D.PaperCharacter|GetSprite _returnvalue) "/Game/Textures/Player/Box/MoveDown.MoveDown")
          (Development|PrintString (Utilities|String|MakeLiteralString (Utilities|String|Append (Utilities|String|MakeLiteralString "Spawned") (Utilities|String|ToString(Integer) _index))))
          (elif (and (not (Utilities|Text|TextIsEmpty (.Name (Utilities|Struct|BreakMonsterStruct _array_element)))) (and (Utilities|Enum|Equal(Enum) (.Name (Utilities|Struct|BreakMonsterStruct _array_element)) (.Monster2 (Utilities|Struct|BreakFormationStruct (Variables|Default|GetBattleFormation)))) (== _index (Utilities|GetLastLetterMacro (.Monster2 (Utilities|Struct|BreakFormationStruct (Variables|Default|GetBattleFormation)))))))
            (goto _label)
            (elif (and (not (Utilities|Text|TextIsEmpty (.Name (Utilities|Struct|BreakMonsterStruct _array_element)))) (and (Utilities|Enum|Equal(Enum) (.Name (Utilities|Struct|BreakMonsterStruct _array_element)) (.Monster3 (Utilities|Struct|BreakFormationStruct (Variables|Default|GetBattleFormation)))) (== _index (Utilities|GetLastLetterMacro (.Monster3 (Utilities|Struct|BreakFormationStruct (Variables|Default|GetBattleFormation)))))))
              (goto _label)
              (elif (and (not (Utilities|Text|TextIsEmpty (.Name (Utilities|Struct|BreakMonsterStruct _array_element)))) (and (Utilities|Enum|Equal(Enum) (.Name (Utilities|Struct|BreakMonsterStruct _array_element)) (.Monster4 (Utilities|Struct|BreakFormationStruct (Variables|Default|GetBattleFormation)))) (== _index (Utilities|GetLastLetterMacro (.Monster4 (Utilities|Struct|BreakFormationStruct (Variables|Default|GetBattleFormation)))))))
                (goto _label)
                (elif (and (not (Utilities|Text|TextIsEmpty (.Name (Utilities|Struct|BreakMonsterStruct _array_element)))) (and (Utilities|Enum|Equal(Enum) (.Name (Utilities|Struct|BreakMonsterStruct _array_element)) (.Monster5 (Utilities|Struct|BreakFormationStruct (Variables|Default|GetBattleFormation)))) (== _index (Utilities|GetLastLetterMacro (.Monster5 (Utilities|Struct|BreakFormationStruct (Variables|Default|GetBattleFormation)))))))
                  (goto _label)))))))))
  ;[1 1 1] Set main camera to the battle camera after camera battle opening sequence
  (EventDispatchers|BindEventtoOnFinished (Variables|/Script/LevelSequence.LevelSequenceActor|GetSequencePlayer (Variables|Default|GetLevelStartSequence)) (delegate Custom|SetBattleCam)))

(fn ConstructionScript)