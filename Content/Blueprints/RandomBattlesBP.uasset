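; Random encounter actor that sends the player into a battle level after enough walking.
; BeginPlay randomizes the encounter threshold around its set value; a non-positive threshold turns encounters off.
; Each Tick with the PlayerCharacter moving horizontally above a minimum speed increments a counter, so timing depends on frame rate.
; At the threshold it resets the counter, disables input, triggers FadeBP's fade-out and opens BattleLevelName without waiting.
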(event EventTick
  (params (DeltaSeconds :type Float%20%28single-precision%29))
  (bind _returnvalue (Game|GetPlayerCharacter 0))
  (if (not (<= (Variables|Default|GetNextEncounterValue) 0.0))
    (Utilities|Casting|CastToPlayerCharacter _returnvalue)
    (if (>= (Math|Vector|VectorLengthXY (Transformation|GetVelocity _returnvalue)) 4e+01)
      (Variables|Default|SetCurrentEncounterValue (+ (Variables|Default|GetCurrentEncounterValue) 1.0))
      (if (>= (+ (Variables|Default|GetCurrentEncounterValue) 1.0) (Variables|Default|GetNextEncounterValue))
        (Variables|Default|SetCurrentEncounterValue 0.0)
        (Input|DisableInput (Game|GetPlayerController 0))
        (bind _outactors (Actor|GetAllActorsOfClass "/Game/Blueprints/FadeBP.FadeBP_C"))
        (Utilities|IsValid (Utilities|Array|Get(acopy) _outactors)
          (:Is%20Valid
            (Default|FadeOut (Utilities|Array|Get(acopy) _outactors)))
          (:Is%20Not%20Valid
            _))
        (Game|OpenLevel(byName) (Variables|Default|GetBattleLevelName))))))

(event EventBeginPlay
  (Variables|Default|SetNextEncounterValue (Math|Random|RandomFloatinRange (- (Variables|Default|GetNextEncounterValue) 1e+02) (+ (Variables|Default|GetNextEncounterValue) 1e+02)))
  (Variables|Default|SetCurrentEncounterValue 0.0))

(fn ConstructionScript)